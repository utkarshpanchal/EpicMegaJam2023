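; GM_Runner is the endless runner's game mode, managing a procedural floor of chained tiles.
; BeginPlay lays the starting tiles and, within the same loop, loads Gears from the GearValue save slot.
; AddChunks spawns a random floor variant at the stored attach point, then takes the new tile's attach point for the next one.
; ExtendFloor adds a tile and destroys the oldest once the count exceeds its limit.
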(event `self.ReceiveBeginPlay`
  (for _ (range (+ (- (`self.Number of Tiles`) 2) 1))
    (`self.AddChunks`)
    (bind _returnvalue (`GameplayStatics.LoadGameFromSlot` "GearValue"))
    (bind _asbp_runner_save_game (cast `/Game/Blueprints/SetupBlueprints/BP_RunnerSaveGame` _returnvalue))
    (set `self.Gears` (`/Game/Blueprints/SetupBlueprints/BP_RunnerSaveGame.GearValue` _asbp_runner_save_game))))

(fn `AddChunks`
  (bind _floor_variants (`self.Floor Variants`))
  (bind _returnvalue (`|SpawnActorFromClass` (`|GetArrayItem` _floor_variants (`KismetMathLibrary.RandomIntegerInRange` 0 (- (`KismetArrayLibrary.Array_Length` _floor_variants) 1))) (`self.Floor Attach Point`) "Undefined" "OverrideRootScale" null null))
  (set `self.Floor Attach Point` (`/Game/Blueprints/Gameplay/Chunks/BP_Chunks.GetAttachPoint` _returnvalue))
  (`KismetArrayLibrary.Array_Add` (`self.Floor Tiles`) _returnvalue))

(fn `ExtendFloor`
  (bind _floor_tiles (`self.Floor Tiles`))
  (bind _output (`|GetArrayItem` _floor_tiles))
  (`self.AddChunks`)
  (if (> (`KismetArrayLibrary.Array_Length` (`self.Floor Tiles`)) (+ (`self.Number of Tiles`) 1))
    (`self.K2_DestroyActor` _output)
    (`KismetArrayLibrary.Array_RemoveItem` _floor_tiles _output)))

(fn `UserConstructionScript`)