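; Main menu pawn that glides from a reference actor's location to its own placed position when play begins, serving as a camera move.
; BeginPlay stores the pawn's location, then MoveCameraPawn plays a timeline whose alpha lerps the location from StartFromActor to that stored point.
; The move only changes location, without sweep, and is skipped when StartFromActor is not valid.
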(event `self.ReceiveBeginPlay`
  (set `self.StartPos` (`self.K2_GetActorLocation`))
  (`self.MoveCameraPawn`))

(event `MoveCameraPawn`
  (bind _startfromactor (`self.StartFromActor`))
  (`/Engine/EditorBlueprintResources/StandardMacros.IsValid` _startfromactor
    (:`Is Valid`
      (bind (_direction _movealpha) (`Timeline|MoveCamera` :!via `PlayFromStart`)
        (:`Update`
          (`self.K2_SetActorLocation` (`KismetMathLibrary.VLerp` (`self.K2_GetActorLocation` _startfromactor) (`self.StartPos`) _movealpha)))))))

(fn `UserConstructionScript`)