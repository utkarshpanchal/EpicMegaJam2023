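; Train box obstacle for a runner game that kills the player on contact and clears barriers that overlap it.
; Overlapping the Box component calls Death on BP_CharacterRunner, then pauses the game after a short delay.
; Both the Box and Patiyu components destroy any overlapping BP_Obstracle_barrier.
; Logic is purely overlap-driven, with no active Tick or BeginPlay behavior.
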(event `self.Box.OnComponentBeginOverlap`
  (params (OverlappedComponent :type "PrimitiveComponent Object Reference") (OtherActor :type "Actor Object Reference") (OtherComp :type "PrimitiveComponent Object Reference") (OtherBodyIndex :type Integer) (bFromSweep :type Boolean) (SweepResult :type "HitResult Structure (by ref)"))
  (`|ExecutionSequence`
    (:`then_0`
      (bind _asbp_character_runner (cast `/Game/Blueprints/SetupBlueprints/BP_CharacterRunner` OtherActor))
      (`/Game/Blueprints/SetupBlueprints/BP_CharacterRunner.Death` _asbp_character_runner)
      (`KismetSystemLibrary.Delay` 2.0)
      (`GameplayStatics.SetGamePaused` true))
    (:`then_1`
      (bind _asbp_obstracle_barrier (cast `/Game/Blueprints/Gameplay/Obstracles/BP_Obstracle_barrier` OtherActor))
      (`self.K2_DestroyActor` _asbp_obstracle_barrier))))

(event `self.patiyu.OnComponentBeginOverlap`
  (params (OverlappedComponent :type "PrimitiveComponent Object Reference") (OtherActor :type "Actor Object Reference") (OtherComp :type "PrimitiveComponent Object Reference") (OtherBodyIndex :type Integer) (bFromSweep :type Boolean) (SweepResult :type "HitResult Structure (by ref)"))
  (bind _asbp_obstracle_barrier (cast `/Game/Blueprints/Gameplay/Obstracles/BP_Obstracle_barrier` OtherActor))
  (`self.K2_DestroyActor` _asbp_obstracle_barrier))

(fn `UserConstructionScript`
  (`parent.UserConstructionScript`))