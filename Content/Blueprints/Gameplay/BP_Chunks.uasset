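; BP_Chunks is a floor chunk for a runner game that extends the track and gradually speeds up the player.
; Any overlap with its Box tells GM_Runner to extend the floor, then slightly multiplies BP_CharacterRunner's walk speed within a clamped range and prints it.
; GetAttachPoint returns the Arrow component's world transform as the chunk's attach point.
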(event `self.Box.OnComponentBeginOverlap`
  (params (OverlappedComponent :type "PrimitiveComponent Object Reference") (OtherActor :type "Actor Object Reference") (OtherComp :type "PrimitiveComponent Object Reference") (OtherBodyIndex :type Integer) (bFromSweep :type Boolean) (SweepResult :type "HitResult Structure (by ref)"))
  ;[1 1 1] Extend floor
  (bind _asgm_runner (cast `/Game/Blueprints/SetupBlueprints/GM_Runner` (`GameplayStatics.GetGameMode`)))
  (`/Game/Blueprints/SetupBlueprints/GM_Runner.ExtendFloor` _asgm_runner)
  ;[1 1 1] change speed
  (bind _asbp_character_runner (cast `/Game/Blueprints/SetupBlueprints/BP_CharacterRunner` (`GameplayStatics.GetPlayerCharacter` 0)))
  (bind _charactermovement (`Character.CharacterMovement` _asbp_character_runner))
  (bind _output_get (set `CharacterMovementComponent.MaxWalkSpeed` (`KismetMathLibrary.FClamp` (* (`CharacterMovementComponent.MaxWalkSpeed` _charactermovement) 1.001) 700.0 1500.0) _charactermovement))
  (`KismetSystemLibrary.PrintString` (`KismetStringLibrary.Conv_DoubleToString` _output_get)))

(fn `GetAttachPoint`
  (returns (ReturnValue :type "Transform Structure"))
  (return (`SceneComponent.K2_GetComponentToWorld` (`self.Arrow`))))

(fn `UserConstructionScript`)