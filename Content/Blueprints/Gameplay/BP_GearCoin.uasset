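; BP_GearCoin is a collectible gear pickup for the runner game, handled entirely on actor overlap.
; When the runner character touches it, it increments the Gears count on GM_Runner, plays a collect sound, destroys itself and has the character update its gear display.
; A second sequence branch destroys the coin when it overlaps a wall obstacle, removing coins that land inside walls.
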(event `self.ReceiveActorBeginOverlap`
  (params (OtherActor :type "Actor Object Reference"))
  (`|ExecutionSequence`
    (:`then_0`
      (bind _asbp_character_runner (cast `/Game/Blueprints/SetupBlueprints/BP_CharacterRunner` OtherActor))
      (bind _asgm_runner (cast `/Game/Blueprints/SetupBlueprints/GM_Runner` (`GameplayStatics.GetGameMode`)))
      (`/Engine/EditorBlueprintResources/StandardMacros.IncrementInt` (`/Game/Blueprints/SetupBlueprints/GM_Runner.Gears` _asgm_runner)
        (:`  `
          (`GameplayStatics.PlaySound2D` "/Game/Assets/Audio/Sounds/Coin/SC_collectcoin-6075_Cue.SC_collectcoin-6075_Cue" 1.0 1.0 0.0 null null)
          (`self.K2_DestroyActor`)
          (`/Game/Blueprints/SetupBlueprints/BP_CharacterRunner.UpdateGears` _asbp_character_runner))))
    (:`then_1`
      (cast `/Game/Blueprints/Gameplay/Obstracles/BP_Obstracle_Child_Wall` OtherActor)
      (`self.K2_DestroyActor`))))

(fn `UserConstructionScript`)